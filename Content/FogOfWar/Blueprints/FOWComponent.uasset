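; FOWComponent is an actor component that defines its owner's footprint, apparently as a fog-of-war occluder.
; On BeginPlay, if CastFOW is set, DefineEdges scales SizeZ by the owner's Z scale and builds the Edges array.
; Edges holds the four corners of a SizeX by SizeY rectangle centered on the owner, transformed to world space and flattened to Z zero.
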(event `self.ReceiveBeginPlay`
  (if (`self.CastFOW`)
    (`self.DefineEdges`)))

(fn `DefineEdges`
  (bind _returnvalue (`Actor.GetTransform` (`self.GetOwner`)))
  (bind _returnvalue_2 (/ (`self.SizeY`) 2.0))
  (bind _returnvalue_3 (/ (`self.SizeX`) 2.0))
  (bind _returnvalue_4 (* _returnvalue_2 -1.0))
  (bind _returnvalue_5 (* _returnvalue_3 -1.0))
  (set `self.SizeZ` (* (.z (.scale _returnvalue)) (`self.SizeZ`)))
  (set `self.Edges` (`|MakeArray` (`KismetMathLibrary.MakeVector` (.x (`KismetMathLibrary.TransformLocation` _returnvalue (`KismetMathLibrary.MakeVector` _returnvalue_3 _returnvalue_4))) (.y (`KismetMathLibrary.TransformLocation` _returnvalue (`KismetMathLibrary.MakeVector` _returnvalue_3 _returnvalue_4)))) (`KismetMathLibrary.MakeVector` (.x (`KismetMathLibrary.TransformLocation` _returnvalue (`KismetMathLibrary.MakeVector` _returnvalue_3 _returnvalue_2))) (.y (`KismetMathLibrary.TransformLocation` _returnvalue (`KismetMathLibrary.MakeVector` _returnvalue_3 _returnvalue_2)))) (`KismetMathLibrary.MakeVector` (.x (`KismetMathLibrary.TransformLocation` _returnvalue (`KismetMathLibrary.MakeVector` _returnvalue_5 _returnvalue_2))) (.y (`KismetMathLibrary.TransformLocation` _returnvalue (`KismetMathLibrary.MakeVector` _returnvalue_5 _returnvalue_2)))) (`KismetMathLibrary.MakeVector` (.x (`KismetMathLibrary.TransformLocation` _returnvalue (`KismetMathLibrary.MakeVector` _returnvalue_5 _returnvalue_4))) (.y (`KismetMathLibrary.TransformLocation` _returnvalue (`KismetMathLibrary.MakeVector` _returnvalue_5 _returnvalue_4)))))))